(event EventTick
  (params (DeltaSeconds :type Float%20%28single-precision%29))
  (if (>= (Variables|Default|GetUp) 1)
    (Transformation|SetActorLocation (+ (Transformation|GetActorLocation) "0,0.100000, 0") false false)))

(fn ConstructionScript)

(fn Up+
  (Variables|Default|SetUp (+ (Variables|Default|GetUp) 1))
  (Development|PrintString "いらっしゃいませー"))

(fn Up-
  (Variables|Default|SetUp (- (Variables|Default|GetUp) 1))
  (Development|PrintString "ありがとうございました。"))

(fn UpGet
  (return (>= (Variables|Default|GetUp) 1)))