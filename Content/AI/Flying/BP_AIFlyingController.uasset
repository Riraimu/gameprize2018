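; AI controller for flying enemies that patrols between points and detects the player robot.
; On BeginPlay it copies patrol points from its BP_AIFlying pawn, seeds the blackboard with wait duration and runs BT_AIFlying.
; PawnSensing writes a sighted Robot_hero_BP to the blackboard's Player key.
; GoToPatrol moves to the current point, advances the wrapping index and re-arms itself on a timer, though nothing here starts it.
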(event OnSeePawn(PawnSensing)
  (params (Pawn :type Pawn%20Object%20Reference))
  (bind _asrobot_hero_bp (Utilities|Casting|CastToRobot_hero_BP Pawn))
  (AI|Components|Blackboard|SetValueasObject (Variables|Default|GetBlackboard self) (Utilities|Name|MakeLiteralName "Player") _asrobot_hero_bp))

(event Custom|GoToPatrol
  (AI|AIMoveTo (Pawn|GetControlledPawn) (CallFunction|GetPatrolLocation) 0 5.0 false
    (:OnSuccess
      (CallFunction|PopPatrolLocation)
      (Utilities|Time|SetTimerbyFunctionName 0 "GoToPatrol" 1.0))))

(event EventBeginPlay
  (bind _asbp_aiflying (Utilities|Casting|CastToBP_AIFlying (Pawn|GetControlledPawn)))
  (Variables|Default|SetAI_PatrolPoints (Variables|/Game/AI/Flying/BP_AIFlying.BP_AIFlying_C|GetPatrolPoints _asbp_aiflying))
  (Class|AIController|UseBlackboard "/Game/AI/Flying/BB_AIFlying.BB_AIFlying")
  (AI|Components|Blackboard|SetValueasFloat (AI|GetBlackboard 0) (Utilities|Name|MakeLiteralName "PatrolWaitDuration") (Variables|/Game/AI/Flying/BP_AIFlying.BP_AIFlying_C|GetPatrolWaitDuration _asbp_aiflying))
  (AI|RunBehaviorTree "/Game/AI/Flying/BT_AIFlying.BT_AIFlying"))

(fn ConstructionScript)

(fn GetPatrolLocation
  (return (Transformation|GetActorLocation (Utilities|Array|Get(acopy) (Variables|Default|GetAI_PatrolPoints) (Variables|Default|GetPatrolIndex)))))

(fn PopPatrolLocation
  (Variables|Default|SetPatrolIndex (Math|Integer|%(Integer) (+ (Variables|Default|GetPatrolIndex) 1) (Utilities|Array|Length (Variables|Default|GetAI_PatrolPoints)))))