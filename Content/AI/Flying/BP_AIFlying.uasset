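; BP_AIFlying is a flying AI Blueprint that provides a line-of-sight check for the player.
; CanSeePlayerPawn traces from the actor along its forward vector for SightLength and tests whether the hit actor has the "Player" tag.
; On a match it sets and returns IsHit and the seen actor.
; The event graph has no active logic and leaves the check unconnected.
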(event EventTick
  (params (DeltaSeconds :type Float%20%28single-precision%29)))

(fn ConstructionScript)

(fn CanSeePlayerPawn
  (bind _returnvalue (Transformation|GetActorLocation))
  (bind (_outhit _returnvalue_2) (Collision|LineTraceByChannel _returnvalue (+ _returnvalue (* (Transformation|GetActorForwardVector) (Variables|Default|GetSightLength))) "TraceTypeQuery3" false 0 "None"))
  (if _returnvalue_2 ; 視線が何かに当たったか
    (if (Actor|ActorHasTag (.HitActor (Collision|BreakHitResult _outhit)) "Player") ; それがプレイヤーだったか?
      (LocalVariables|SetIsHit (Actor|ActorHasTag (.HitActor (Collision|BreakHitResult _outhit)) "Player"))
      (LocalVariables|SetHitActor (.HitActor (Collision|BreakHitResult _outhit)))))
  (return (LocalVariables|GetIsHit) (LocalVariables|GetHitActor)))