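; AI controller for BP_AICharacter1, a ground enemy that patrols and detects the player.
; On BeginPlay it copies the pawn's patrol points and wait duration, sets up its Blackboard and runs BT_AICharacter1.
; Pawn sensing writes a seen Robot_hero_BP to the Player key.
; A separate GoToPatrol event loops through patrol points via AIMoveTo and a timer, but nothing in this graph starts it.
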(event OnSeePawn(PawnSensing)
  (params (Pawn :type Pawn%20Object%20Reference))
  (bind _asrobot_hero_bp (Utilities|Casting|CastToRobot_hero_BP Pawn))
  (AI|Components|Blackboard|SetValueasObject (Variables|Default|GetBlackboard self) (Utilities|Name|MakeLiteralName "Player") _asrobot_hero_bp))

(event Custom|GoToPatrol
  ;[1 1 1] GoToPatrol
  (AI|AIMoveTo (Pawn|GetControlledPawn) (CallFunction|GetPatrolLocation) 0 5.0 false
    (:OnSuccess
      (CallFunction|PopPatrolLocation)
      (Utilities|Time|SetTimerbyFunctionName 0 "GoToPatrol" 1.0))))

(event EventBeginPlay
  ;[1 1 1] BeginPlay
  (bind _asbp_aicharacter_1 (Utilities|Casting|CastToBP_AICharacter1 (Pawn|GetControlledPawn)))
  (Variables|Default|SetAI_PatrolPoints (Variables|/Game/AI/Ground/BP_AICharacter1.BP_AICharacter1_C|GetPatrolPoints _asbp_aicharacter_1))
  (Class|AIController|UseBlackboard "/Game/AI/Ground/AICharacter1_BlackBoard.AICharacter1_BlackBoard")
  (AI|Components|Blackboard|SetValueasFloat (AI|GetBlackboard 0) (Utilities|Name|MakeLiteralName "PatrolWaitDuration") (Variables|/Game/AI/Ground/BP_AICharacter1.BP_AICharacter1_C|GetPatrolWaitDuration _asbp_aicharacter_1))
  (AI|RunBehaviorTree "/Game/AI/Ground/BT_AICharacter1.BT_AICharacter1"))

(fn ConstructionScript)

(fn GetPatrolLocation
  (return (Transformation|GetActorLocation (Utilities|Array|Get(acopy) (Variables|Default|GetAI_PatrolPoints) (Variables|Default|GetPatrol%20Index)))))

(fn PopPatrolLocation
  (Variables|Default|SetPatrol%20Index (Math|Integer|%(Integer) (+ (Variables|Default|GetPatrol%20Index) 1) (Utilities|Array|Length (Variables|Default|GetAI_PatrolPoints)))))