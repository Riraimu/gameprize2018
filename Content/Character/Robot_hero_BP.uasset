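; Player robot hero Character with camera-relative movement, gamepad turning, jumping, and a switchable input/output mode.
; A gamepad face button or U toggles PlayerM unless Hitcode is set, and Tick swaps the mesh material to match.
; BeginPlay adds the HUD, and OpenMenu replaces it with a UI-only pause menu.
; Small functions expose PlayerM, flip Hitcode and clear TensouDataP.
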(event EventTick
  (params (DeltaSeconds :type Float%20%28single-precision%29))
  ;[1 1 1] モードによるカラーチェンジ
  (if (Variables|Default|GetPlayer_M)
    (Rendering|Material|SetMaterial (Variables|Character|GetMesh) 0 "/Game/Character/blinn5.blinn5")
    (else
      (Rendering|Material|SetMaterial (Variables|Character|GetMesh) 0 "/Game/Character/binn6.binn6"))))

(event EventBeginPlay
  ;[1 1 1] HUD(HP&EXゲージを作成)
  (bind _returnvalue (UserInterface|CreateWidget "/Game/Blueprints/HUD.HUD_C"))
  (bind _output_get (Variables|Default|SetHUDReference _returnvalue))
  (UserInterface|Viewport|AddtoViewport _output_get 0))

(event Input|ActionEvents|InputActionJump
  (params (Key :type Key%20Structure))
  ;[1 1 1] ジャンプ
  (:Pressed
    (Character|Jump)
    (Variables|Default|SetJumpButtonDown (Character|CanJump))
    (bind _ascharacter_movement_component (Utilities|Casting|CastToCharacterMovementComponent (Pawn|GetMovementComponent) :!label _label))
    (if (> (Math|Vector|VectorLength (Variables|/Script/Engine.MovementComponent|GetVelocity _ascharacter_movement_component)) 0.0)
      (Variables|/Script/Engine.CharacterMovementComponent|SetJumpZVelocity _ascharacter_movement_component 7e+02)
      (else
        (Variables|/Script/Engine.CharacterMovementComponent|SetJumpZVelocity _ascharacter_movement_component 7e+02))))
  (:Released
    (Character|StopJumping)
    (Variables|Default|SetJumpButtonDown false)
    (goto _label)))

(event Input|ActionEvents|InputActionOpenMenu
  (params (Key :type Key%20Structure))
  ;[1 1 1] 一時停止画面を表示
  (:Pressed
    (bind _returnvalue (UserInterface|CreateWidget "/Game/Menu/PauseMenu.PauseMenu_C"))
    (UserInterface|Viewport|AddtoViewport _returnvalue 0)
    (Input|SetInputModeUIOnly (Game|GetPlayerController 0) (Variables|/Game/Menu/PauseMenu.PauseMenu_C|GetEnergyDataLv1 _returnvalue) "DoNotLock")
    ;[1 1 1] HUD非表示
    (Widget|RemovefromParent (Variables|Default|GetHUDReference))))

(event Input|AxisEvents|InputAxisMoveForward
  (params (AxisValue :type Float%20%28single-precision%29))
  ;[1 1 1] キャラクターの移動
  (Pawn|Input|AddMovementInput (Math|Vector|GetForwardVector (Math|Rotator|MakeRotator 0.0 0.0 (.Yaw (Math|Rotator|BreakRotator (Pawn|GetControlRotation :!class /Script/Engine.Pawn))))) AxisValue false))

(event Input|AxisEvents|InputAxisMoveRight
  (params (AxisValue :type Float%20%28single-precision%29))
  ;[1 1 1] キャラクターの移動
  (Pawn|Input|AddMovementInput (Math|Vector|GetRightVector (Math|Rotator|MakeRotator 0.0 0.0 (.Yaw (Math|Rotator|BreakRotator (Pawn|GetControlRotation :!class /Script/Engine.Pawn))))) AxisValue false))

(event Input|AxisEvents|InputAxisTurnRate
  (params (AxisValue :type Float%20%28single-precision%29))
  ;[1 1 1] ゲームパッド
  (Pawn|Input|AddControllerYawInput (* AxisValue (Variables|Default|GetBaseTurnRate) (Utilities|Time|GetWorldDeltaSeconds))))

(event Input|GamepadEvents|GamepadFaceButtonTop
  (params (Key :type Key%20Structure))
  ;[1 1 1] 主人公モード切替
  (:Pressed
    (if (not (Variables|Default|GetHitcode)) ; コードの当たってるか？判定
      (if (Variables|Default|GetPlayer_M) ; 現在のPlayerMの判定
        (Variables|Default|SetPlayer_M false)
        (Development|PrintString "インプットモード")
        (else
          (Variables|Default|SetPlayer_M true)
          (Development|PrintString "アウトプットモード"))))))

(event Input|KeyboardEvents|U
  (params (Key :type Key%20Structure))
  ;[1 1 1] 主人公モード切替
  (:Pressed
    (if (not (Variables|Default|GetHitcode)) ; コードの当たってるか？判定
      (if (Variables|Default|GetPlayer_M) ; 現在のPlayerMの判定
        (Variables|Default|SetPlayer_M false)
        (Development|PrintString "インプットモード")
        (else
          (Variables|Default|SetPlayer_M true)
          (Development|PrintString "アウトプットモード"))))))

(fn ConstructionScript)

(fn GetPM
  (return (Variables|Default|GetPlayer_M)))

(fn FlagHC
  (if (Variables|Default|GetHitcode)
    (Variables|Default|SetHitcode false)
    (else
      (Variables|Default|SetHitcode true))))

(fn SetTDP
  (Variables|Default|Settensou_data_p false))